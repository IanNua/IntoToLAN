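; Custom Game State for a session that picks a random player from the PlayerArray and reports it through debug prints.
; RunRandom calls ServerPickRandom, which rolls an index bounded by the array's last index, so the final player is never chosen when several exist.
; It then calls ClientPickRandom, which loops over the players, printing the chosen one or "Normal Player" for others.
; BeginPlay and the PlayerName OnRep are empty.
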(event `self.ReceiveBeginPlay`)

(event `RunRandom`
  (`self.ServerPickRandom`))

(event `ServerPickRandom`
  (for (_ _array_index) (`self.PlayerArray`)
    _)
  (bind _output_get (set `self.RandomPlayerIndex` (`KismetMathLibrary.RandomInteger` _array_index)))
  (`KismetSystemLibrary.PrintString` (`KismetTextLibrary.Conv_TextToString` (`|FormatText` "Random Player Index {RPI}" _output_get)) true true (struct :`R` 1.0 :`G` 0.20158 :`A` 1.0))
  (`self.ClientPickRandom`))

(event `ClientPickRandom`
  (bind _playerarray (`self.PlayerArray`))
  (for (_ _array_index) _playerarray
    (if (== (`self.RandomPlayerIndex`) _array_index)
      (`KismetSystemLibrary.PrintString` (`KismetTextLibrary.Conv_TextToString` (`|FormatText` "Random Player : {sa}" (`|GetArrayItem` _playerarray _array_index))))
      (else
        (`KismetSystemLibrary.PrintString` "Normal Player")))))

(fn `OnRep_PlayerName`)

(fn `UserConstructionScript`)