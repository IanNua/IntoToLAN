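; Test actor that runs a countdown and prints its progress as debug strings.
; BeginPlay starts a looping one-second timer that decrements Time, prints the current value, then pauses itself and prints "GAME OVER" once it reaches zero or below.
; Time has an OnRep function, but it is empty, and a CallTestEventTimer call is left unconnected.
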(event `self.ReceiveBeginPlay`
  (`self.Start Timer`))

(event `Start Timer`
  (`KismetSystemLibrary.PrintString` "Start Timer")
  (bind _returnvalue (`KismetSystemLibrary.K2_SetTimerDelegate` (delegate `Set Timer`) 1.0 true)))

(event `Set Timer`
  (bind _output_get (set `self.Time` (- (`self.Time`) 1)))
  (`KismetSystemLibrary.PrintString` (`KismetStringLibrary.Concat_StrStr` "Current Time Is :: " (`KismetStringLibrary.Conv_IntToString` _output_get)))
  (if (<= _output_get 0)
    (`KismetSystemLibrary.K2_PauseTimerHandle` (stale `Start Timer` _returnvalue))
    (`KismetSystemLibrary.PrintString` "GAME OVER")))

(fn `OnRep_Time`)

(fn `UserConstructionScript`)