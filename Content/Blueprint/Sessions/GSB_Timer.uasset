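; GSB_Timer is a session timer, apparently a Game State Blueprint, that runs a match countdown once players join.
; CheckPlayerJoined loops over PlayerArray and calls ServerTime at index 1, meaning a second player is present.
; ServerTime starts a looping one-second timer that decrements Time, pausing it at zero with an "END GAME" debug print.
; Time has an empty OnRep function, and all feedback is debug prints.
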(event `CheckPlayerJoined`
  ;[1 1 1] Checks players joined
  (for (_ _array_index) (`self.PlayerArray`)
    (`KismetSystemLibrary.PrintString` (`KismetStringLibrary.Concat_StrStr` "How many Players in Project : " (`KismetStringLibrary.Conv_IntToString` _array_index)) true true (struct :`R` 1.0 :`B` 0.559439 :`A` 1.0))
    (if (== _array_index 1)
      (`self.ServerTime`))))

(event `self.ReceiveBeginPlay`)

(event `ServerTime`
  ;[1 1 1] Uses Timer over Server
  (`KismetSystemLibrary.PrintString` "START TIMER" true true (struct :`R` 1.0 :`B` 0.726131 :`A` 1.0))
  (bind _returnvalue (`KismetSystemLibrary.K2_SetTimerDelegate` (delegate `CountDownTimer`) 1.0 true)))

(event `CountDownTimer`
  ;[1 1 1] Uses Timer over Server
  (bind _output_get (set `self.Time` (- (`self.Time`) 1)))
  (`KismetSystemLibrary.PrintString` (`KismetStringLibrary.Concat_StrStr` "CurrentTime:" (`KismetStringLibrary.Conv_IntToString` _output_get)) true true (struct :`R` 1.0 :`B` 0.785793 :`A` 1.0))
  (if (<= _output_get 0)
    (`KismetSystemLibrary.K2_PauseTimerHandle` (stale `ServerTime` _returnvalue))
    (`KismetSystemLibrary.PrintString` "END GAME" true true (struct :`R` 1.0 :`B` 0.156789 :`A` 1.0))))

(fn `OnRep_Time`)

(fn `UserConstructionScript`)